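; BP_LevelDetector is a trigger actor that moves the player on to the next level when they overlap it.
; On overlap with BP_PlayerFPS, it compares the current level name against stored names for levels one to three and opens the following level.
; Any other level name, presumably the fourth level, falls through to open the win map.
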(event Collision|EventActorBeginOverlap
  (params (OtherActor :type Actor%20Object%20Reference))
  (Utilities|Casting|CastToBP_PlayerFPS OtherActor)
  (bind _returnvalue (Game|GetCurrentLevelName true))
  (bind _output_get (Variables|Default|SetCurrentLevelname _returnvalue))
  (if (Utilities|Enum|Equal(Enum) _output_get (Variables|Default|GetLevelOneName))
    (Game|OpenLevel(byObjectReference) "/Game/Maps/LevelTwo.LevelTwo")
    (elif (Utilities|Enum|Equal(Enum) (Variables|Default|GetCurrentLevelname) (Variables|Default|GetLevelTwoName))
      (Game|OpenLevel(byObjectReference) "/Game/Maps/LevelThree.LevelThree")
      (elif (Utilities|Enum|Equal(Enum) (Variables|Default|GetCurrentLevelname) (Variables|Default|GetLevelThreeName))
        (Game|OpenLevel(byObjectReference) "/Game/Maps/LevelFour.LevelFour")
        (else
          (Game|OpenLevel(byObjectReference) "/Game/Maps/WinMap.WinMap"))))))

(fn ConstructionScript)