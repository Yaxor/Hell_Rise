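; BP_PlayerFPS is the first-person player Blueprint, which syncs the player's CurrentLife with the health stored in BP_HellRiseGameInstance.
; Shortly after BeginPlay, a timer calls SetInitialCurrentLife to cache the game instance and load the saved health.
; OnUpdateCurrentLifeGI writes CurrentLife back to it; if the cached reference is invalid, it only re-caches the instance without writing the value.
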(event EventBeginPlay
  ;[0.2023 0 1] Set the current CurrentLife
  (Utilities|Time|SetTimerbyFunctionName self "SetInitialCurrentLife" 0.1))

(event EventOnUpdateCurrentLifeGI
  ;[1 0 0] Update CurrentLife in GameInstance
  (Utilities|IsValid (Variables|Default|GetHellRiseGameInstance)
    (:Is%20Valid
      (Variables|/Game/Blueprints/GameFramework/BP_HellRiseGameInstance.BP_HellRiseGameInstance_C|SetPlayerCurrentHealth (Variables|Default|GetHellRiseGameInstance) (Variables|Default|GetCurrentLife)))
    (:Is%20Not%20Valid
      (bind _asbp_hell_rise_game_instance (Utilities|Casting|CastToBP_HellRiseGameInstance (Game|GetGameInstance)))
      (Variables|Default|SetHellRiseGameInstance _asbp_hell_rise_game_instance))))

(fn ConstructionScript)

(fn SetInitialCurrentLife
  (bind _asbp_hell_rise_game_instance (Utilities|Casting|CastToBP_HellRiseGameInstance (Game|GetGameInstance)))
  (bind _output_get (Variables|Default|SetHellRiseGameInstance _asbp_hell_rise_game_instance))
  (Variables|Default|SetCurrentLife (Variables|/Game/Blueprints/GameFramework/BP_HellRiseGameInstance.BP_HellRiseGameInstance_C|GetPlayerCurrentHealth _output_get)))