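; FPS player controller that owns the player's HUD and pause menu widgets.
; Separate events create both widgets, adding the pause menu hidden with a reference back to the controller.
; Pass-through events forward life, ammo and status feedback (damage, hurt, freeze, stun, death, speed-up) to the HUD after validity checks.
; PausetheGame toggles game pause, menu visibility, focus and mouse cursor, also hiding the options panel on resume.
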(event EventGetDamageFeedback
  (bind _playerhud (Variables|Default|GetPlayerHUD))
  ;[1 0 0] Hurt Feedback
  (Utilities|IsValid _playerhud
    (:Is%20Valid
      (Default|GetDamageFeedback _playerhud))))

(event EventHurtFeedback
  (bind _playerhud (Variables|Default|GetPlayerHUD))
  ;[1 0 0] Hurt Feedback
  (Utilities|IsValid _playerhud
    (:Is%20Valid
      (Default|HurtFeedback _playerhud))))

(event EventDeathFeedbackon
  (bind _playerhud (Variables|Default|GetPlayerHUD))
  ;[1 0 0] DeathFeedback
  (Utilities|IsValid _playerhud
    (:Is%20Valid
      (Default|DeathFeedBackon _playerhud))))

(event EventStunFeedbackon
  (bind _playerhud (Variables|Default|GetPlayerHUD))
  ;[1 0.2289 0] Stun Feedback
  (Utilities|IsValid _playerhud
    (:Is%20Valid
      (Default|StunFeedbackon _playerhud))))

(event EventStunFeedbackOff
  (bind _playerhud (Variables|Default|GetPlayerHUD))
  ;[1 0.2289 0] Stun Feedback
  (Utilities|IsValid _playerhud
    (:Is%20Valid
      (Default|StunFeedbackOff _playerhud))))

(event EventSpeedUpFeedbackon
  (bind _playerhud (Variables|Default|GetPlayerHUD))
  ;[0 1 0.08126] SpeedUp Feedback
  (Utilities|IsValid _playerhud
    (:Is%20Valid
      (Default|SpeedUpFeedbackon _playerhud))))

(event EventSpeedUpFeedbackOff
  (bind _playerhud (Variables|Default|GetPlayerHUD))
  ;[0 1 0.08126] SpeedUp Feedback
  (Utilities|IsValid _playerhud
    (:Is%20Valid
      (Default|SpeedUpFeedbackOff _playerhud))))

(event EventAddUItoViewport
  ;[0.1175 0.5514 1] Create UI
  (bind _returnvalue (UserInterface|CreateWidget "/Game/Widgets/WBP_PlayerHUD.WBP_PlayerHUD_C" self))
  (bind _output_get (Variables|Default|SetPlayerHUD _returnvalue))
  (UserInterface|Viewport|AddtoViewport _output_get 0))

(event EventUpdateLifePercentHUD
  (params (LifeValuePercent :type Float%20%28single-precision%29))
  (bind _playerhud (Variables|Default|GetPlayerHUD))
  ;[0.1393 1 0.08227] Update PlayerLifeBar
  (Utilities|IsValid _playerhud
    (:Is%20Valid
      (Default|UpdatePlayerLifeBar _playerhud LifeValuePercent))))

(event EventUpdateAmmoAmountHUD
  (params (AmmoAmount :type Byte :default 0) (MagAmount :type Byte :default 0))
  (bind _playerhud (Variables|Default|GetPlayerHUD))
  ;[0.9647 0.521 0] Update Ammo and Mags
  (Utilities|IsValid _playerhud
    (:Is%20Valid
      (Default|UpdateAmmo _playerhud AmmoAmount MagAmount))))

(event EventHurtFeedbackOff
  (bind _playerhud (Variables|Default|GetPlayerHUD))
  ;[1 0 0] Hurt Feedback
  (Utilities|IsValid _playerhud
    (:Is%20Valid
      (Default|HurtFeedbackOff _playerhud))))

(event EventPausetheGame
  (bind _pausehud (Variables|Default|GetPauseHUD))
  (bind _pausehud_2 (Variables|Default|GetPauseHUD))
  ;[0.1134 0 1] Set PauseHud On Screen
  (if (Variables|Default|GetbGameIsOnPause)
    (bind _output_get (Variables|Default|SetbGameIsOnPause false))
    (Game|SetGamePaused _output_get)
    (Class|WidgetBlueprintLibrary|SetFocustoGameViewport)
    (Widget|SetVisibility _pausehud "Hidden")
    (Widget|SetVisibility (Variables|/Game/Widgets/WBP_PauseMenu.WBP_PauseMenu_C|GetOptionsPanel _pausehud) "Hidden")
    (Variables|Default|SetbShowMouseCursor false)
    (else
      (bind _output_get_2 (Variables|Default|SetbGameIsOnPause true))
      (Game|SetGamePaused _output_get_2)
      (Widget|SetVisibility _pausehud_2 "Visible")
      (Widget|SetFocus _pausehud_2)
      (Variables|Default|SetbShowMouseCursor true))))

(event EventFreezeFeedbackon
  (bind _playerhud (Variables|Default|GetPlayerHUD))
  ;[0 1 0.9194] Freeze Feedback
  (Utilities|IsValid _playerhud
    (:Is%20Valid
      (Default|FreezeFeedbackon _playerhud))))

(event EventAddPauseMenutoViewport
  ;[0.2448 0.2448 0.2448] Create PauseMenu
  (bind _returnvalue (UserInterface|CreateWidget "/Game/Widgets/WBP_PauseMenu.WBP_PauseMenu_C" self))
  (bind _output_get (Variables|Default|SetPauseHUD _returnvalue))
  (Variables|/Game/Widgets/WBP_PauseMenu.WBP_PauseMenu_C|SetController _output_get self)
  (Widget|SetVisibility (Variables|Default|GetPauseHUD) "Hidden")
  (UserInterface|Viewport|AddtoViewport (Variables|Default|GetPauseHUD) 0)
  (Class|WidgetBlueprintLibrary|SetFocustoGameViewport))

(event EventFreezeFeedbackOff
  (bind _playerhud (Variables|Default|GetPlayerHUD))
  ;[0 1 0.9194] Freeze Feedback
  (Utilities|IsValid _playerhud
    (:Is%20Valid
      (Default|FreezeFeedbackOff _playerhud))))

(fn ConstructionScript)